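; Placeable candle furniture that can be lit and snuffed, using four particle system components.
; Its Interact function flips the OnOff state, activating or deactivating all four particle systems together, and always returns false.
; When a BP_Pawn's capsule enters the Box, the Interact component's visibility is set to the current OnOff value, with no end-overlap handling.
; Some leftover toggle and activation nodes in the event graph are unconnected.
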(event `self.Box.OnComponentBeginOverlap`
  (params (OverlappedComponent :type "PrimitiveComponent Object Reference") (OtherActor :type "Actor Object Reference") (OtherComp :type "PrimitiveComponent Object Reference") (OtherBodyIndex :type Integer) (bFromSweep :type Boolean) (SweepResult :type "HitResult Structure (by ref)"))
  (cast `/Game/Player/BP_Pawn` OtherActor)
  (cast `CapsuleComponent` OtherComp)
  (`SceneComponent.SetVisibility` (`self.  interact`) (`self.On Off`) false))

(fn `Interact`
  (returns (succes :type Boolean))
  (bind _particlesystem (`self.ParticleSystem`))
  (if (`self.On Off`)
    (`ActorComponent.Deactivate` _particlesystem)
    (`ActorComponent.Deactivate` (`self.ParticleSystem1`))
    (`ActorComponent.Deactivate` (`self.ParticleSystem2`))
    (`ActorComponent.Deactivate` (`self.ParticleSystem3`))
    (set `self.On Off` false)
    (else
      (`ActorComponent.Activate` _particlesystem false)
      (`ActorComponent.Activate` (`self.ParticleSystem1`) false)
      (`ActorComponent.Activate` (`self.ParticleSystem2`) false)
      (`ActorComponent.Activate` (`self.ParticleSystem3`) false)
      (set `self.On Off` true)))
  (return false))

(fn `UserConstructionScript`
  (`parent.UserConstructionScript`))